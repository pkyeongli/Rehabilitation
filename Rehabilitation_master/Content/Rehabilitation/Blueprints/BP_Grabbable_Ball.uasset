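; Grabbable rehabilitation-game ball that displays one of several food meshes, chosen by FoodNumber at BeginPlay.
; MoveStart makes it glide via VInterpTo on Tick toward a raised goal position, destroying itself when close, while Grabbed stops the motion.
; TestThrow releases it through GrabComponentBall with a given velocity, and GoalBall gives it a short lifespan.
; On destruction it tells every BP_GameController to spawn another ball; mesh hits only print the other actor's name.
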(event `self.ReceiveBeginPlay`
  (`self.SetMeshToNumber` (`self.FoodNumber`)))

(event `self.ReceiveTick`
  (params (DeltaSeconds :type "Float (single-precision)"))
  (bind _returnvalue (`self.K2_GetActorLocation`))
  (bind _goalposition (`self.GoalPosition`))
  (if (`self.IsEnable`)
    (`self.K2_SetActorLocation` (`KismetMathLibrary.VInterpTo` _returnvalue _goalposition DeltaSeconds (`self.speed`)))
    (if (<= (`KismetMathLibrary.Vector_Distance` _returnvalue _goalposition) 25.0)
      (`self.K2_DestroyActor`))))

(event `MoveStart`
  (params (goalposition :type "Vector Structure"))
  (set `self.IsEnable` true)
  (set `self.GoalPosition` (+ goalposition (0.0 0.0 75.0))))

(event `/Game/Rehabilitation/Blueprints/BPI_Grab.Grabbed`
  (set `self.IsEnable` false))

(event `TestThrow`
  (params (velocity :type "Vector Structure"))
  (`/Game/Rehabilitation/Blueprints/GrabComponent.TryRelease` (`self.GrabComponent_Ball`) velocity))

(event `GoalBall`
  (`self.SetLifeSpan` 0.5))

(event `self.ReceiveDestroyed`
  (bind _outactors (`GameplayStatics.GetAllActorsOfClass` "/Game/Rehabilitation/Blueprints/BP_GameController.BP_GameController_C"))
  (for _array_element _outactors
    (`/Game/Rehabilitation/Blueprints/BP_GameController.SpawnBall` _array_element)))

(event `self.StaticMesh.OnComponentHit`
  (params (HitComponent :type "PrimitiveComponent Object Reference") (OtherActor :type "Actor Object Reference") (OtherComp :type "PrimitiveComponent Object Reference") (NormalImpulse :type "Vector Structure") (Hit :type "HitResult Structure (by ref)"))
  (`KismetSystemLibrary.PrintString` (`KismetSystemLibrary.GetDisplayName` OtherActor)))

(fn `SetMeshToNumber`
  (params (number :type Integer))
  (bind _staticmesh (`self.StaticMesh`))
  (switch `int` number
    (:`Default`
      (`StaticMeshComponent.SetStaticMesh` _staticmesh "/Game/Fantastic_Village_Pack/meshes/props/food/SM_PROP_food_cauliflower.SM_PROP_food_cauliflower" :!label _label))
    (:`0`
      (goto _label))
    (:`1`
      (`StaticMeshComponent.SetStaticMesh` _staticmesh "/Game/Fantastic_Village_Pack/meshes/props/food/SM_PROP_food_pumpkin_03.SM_PROP_food_pumpkin_03"))
    (:`2`
      (`StaticMeshComponent.SetStaticMesh` _staticmesh "/Game/Fantastic_Village_Pack/meshes/props/food/SM_PROP_food_watermelon_01.SM_PROP_food_watermelon_01"))
    (:`3`
      (`StaticMeshComponent.SetStaticMesh` _staticmesh "/Game/Fantastic_Village_Pack/meshes/props/food/SM_PROP_food_fish_02.SM_PROP_food_fish_02"))
    (:`4`
      (`StaticMeshComponent.SetStaticMesh` _staticmesh "/Game/Fantastic_Village_Pack/meshes/props/food/SM_PROP_food_meat_06.SM_PROP_food_meat_06"))))

(fn `UserConstructionScript`)