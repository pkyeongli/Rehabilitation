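; BP_Ring is a ring target in a rehabilitation game that scores when a grabbable ball passes down through it.
; A ball ending overlap with the cylinder at or below the ring's center counts as a goal and is notified.
; A goal spawns explosion and sound effects, notifies every BP_GameController, and destroys the ring shortly after.
; ApplyScale resizes the cylinder's X and Y relative to its starting scale, keeping Z fixed.
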(event `self.ReceiveBeginPlay`
  (set `self.InitScale` (`SceneComponent.K2_GetComponentScale` (`self.Cylinder`))))

(event `self.Cylinder.OnComponentEndOverlap`
  (params (OverlappedComponent :type "PrimitiveComponent Object Reference") (OtherActor :type "Actor Object Reference") (OtherComp :type "PrimitiveComponent Object Reference") (OtherBodyIndex :type Integer))
  (bind _asbp_grabbable_ball (cast `/Game/Rehabilitation/Blueprints/BP_Grabbable_Ball` OtherActor))
  (if (<= (.z (`KismetMathLibrary.GetDirectionUnitVector` (`self.K2_GetActorLocation`) (`self.K2_GetActorLocation` _asbp_grabbable_ball))) 0.0)
    (`self.Goal`)
    (`/Game/Rehabilitation/Blueprints/BP_Grabbable_Ball.GoalBall` _asbp_grabbable_ball)))

(event `Goal`
  (bind _returnvalue (`self.K2_GetActorLocation`))
  (`GameplayStatics.SpawnEmitterAtLocation` "/Game/ExampleContent/Blueprint_Communication/Effects/P_Explosion_Fireball.P_Explosion_Fireball" _returnvalue)
  (`GameplayStatics.SpawnSoundAtLocation` "/Engine/VREditor/Sounds/VR_confirm_Cue.VR_confirm_Cue" _returnvalue (struct) 1.0 1.0 0.0 null null)
  (`self.SetLifeSpan` 0.5)
  (bind _outactors (`GameplayStatics.GetAllActorsOfClass` "/Game/Rehabilitation/Blueprints/BP_GameController.BP_GameController_C"))
  (for _array_element _outactors
    (message `/Game/Rehabilitation/Blueprints/BPI_Controller.GoalRing` _array_element)))

(event `ApplyScale`
  (params (ScaleValue :type "Float (double-precision)" :default 1.0))
  (bind (_initscale_x _initscale_y _initscale_z) (`KismetMathLibrary.BreakVector` (`self.InitScale`)))
  (bind _output_get (set `self.CurrentScale` ScaleValue))
  (`SceneComponent.SetWorldScale3D` (`self.Cylinder`) (`KismetMathLibrary.MakeVector` (* _initscale_x _output_get) (* _initscale_y _output_get) _initscale_z)))

(fn `ChangeScaleMagnification`)

(fn `UserConstructionScript`)