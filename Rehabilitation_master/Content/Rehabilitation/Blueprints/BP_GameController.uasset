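; Game controller actor for a VR ball-and-ring round, with an animated dragon that reacts to the player's results.
; StartGame resets the VR game instance, spawns a scaled ring facing the player and sends a short-lived grabbable food ball toward them.
; GoalRing records a success and respawns the ring; each SpawnBall call plays a sick reaction after a miss or ends the round when NextTime signals, celebrating or dying against GoalCount.
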(event `PlayIdle`
  (`SkeletalMeshComponent.PlayAnimation` (`self.SkeletalMesh`) "/Game/Tiny_Dragon/Animations/Anim_Dra_Fly.Anim_Dra_Fly" true :!label _label))

(event `/Game/Rehabilitation/SR/SR_Minigame/BPI_ButtonPressed.ButtonPressed`
  (`self.StartGame`))

(event `self.ReceiveBeginPlay`
  (goto _label))

(event `SpawnBall`
  (bind _vrgameinstance (`/Game/Rehabilitation/Blueprints/MiscUtils/MiscUtils_BP.GetVRGameInstance`))
  (if (`/Game/Rehabilitation/Blueprints/VRGameInstance_BP.IsGameStart` _vrgameinstance)
    (bind _isfinish (`/Game/Rehabilitation/Blueprints/VRGameInstance_BP.NextTime` _vrgameinstance))
    (if _isfinish
      (`self.FinishGame`)
      (else
        (`|ExecutionSequence`
          (:`then_0`
            (if (`self.IsPassRing`)
              (set `self.IsPassRing` false)
              (else
                (`SkeletalMeshComponent.PlayAnimation` (`self.SkeletalMesh`) "/Game/Tiny_Dragon/Animations/Anim_Dra_Sick.Anim_Dra_Sick" false)
                (`KismetSystemLibrary.Delay` 1.4)
                (`self.PlayIdle`))))
          (:`then_1`
            (`KismetSystemLibrary.Delay` 2.0)
            (bind _returnvalue (`|SpawnActorFromClass` "/Game/Rehabilitation/Blueprints/BP_Grabbable_Ball.BP_Grabbable_Ball_C" (`KismetMathLibrary.MakeTransform` (`SceneComponent.K2_GetComponentLocation` (`self.BallSpawnPosition`))) "AlwaysSpawn" "OverrideRootScale" self (`KismetMathLibrary.RandomIntegerInRange` 0 4) null))
            (`PrimitiveComponent.SetEnableGravity` (`/Game/Rehabilitation/Blueprints/BP_Grabbable_Ball.StaticMesh` _returnvalue) false)
            (`/Game/Rehabilitation/Blueprints/BP_Grabbable_Ball.MoveStart` _returnvalue (`SceneComponent.K2_GetComponentLocation` (`self.PlayerPosition`)))
            (`self.SetLifeSpan` _returnvalue 5.0)))))))

(event `SpawnRing`
  (bind _returnvalue (`SceneComponent.K2_GetComponentLocation` (`self.RingPosition`)))
  (if (`/Game/Rehabilitation/Blueprints/VRGameInstance_BP.IsGameStart` (`/Game/Rehabilitation/Blueprints/MiscUtils/MiscUtils_BP.GetVRGameInstance`))
    (bind _ringobject (`self.RingObject`)
      (:`then`
        (`self.K2_DestroyActor` _ringobject))
      (:`else`
        _))
    (bind _returnvalue_2 (`|SpawnActorFromClass` "/Game/Rehabilitation/Blueprints/BP_Ring.BP_Ring_C" (`KismetMathLibrary.MakeTransform` _returnvalue (`KismetMathLibrary.FindLookAtRotation` _returnvalue (`SceneComponent.K2_GetComponentLocation` (`self.PlayerPosition`)))) "AlwaysSpawn" "OverrideRootScale" self null))
    (bind _output_get (set `self.RingObject` _returnvalue_2))
    (`/Game/Rehabilitation/Blueprints/BP_Ring.ApplyScale` _output_get (`/Game/Rehabilitation/Blueprints/VRGameInstance_BP.GetRingScaleValue` (`/Game/Rehabilitation/Blueprints/MiscUtils/MiscUtils_BP.GetVRGameInstance`)))))

(event `/Game/Rehabilitation/Blueprints/BPI_Controller.GoalRing`
  (set `self.IsPassRing` true)
  (`SkeletalMeshComponent.PlayAnimation` (`self.SkeletalMesh`) "/Game/Tiny_Dragon/Animations/Anim_Dra_Eat.Anim_Dra_Eat" false)
  (`KismetSystemLibrary.Delay` 1.0)
  (`SkeletalMeshComponent.PlayAnimation` (`self.SkeletalMesh`) "/Game/Tiny_Dragon/Animations/Anim_Dra_Eat.Anim_Dra_Eat" false)
  (`KismetSystemLibrary.Delay` 1.0)
  (`SkeletalMeshComponent.PlayAnimation` (`self.SkeletalMesh`) "/Game/Tiny_Dragon/Animations/Anim_Dra_Fly_Fire.Anim_Dra_Fly_Fire" true)
  (`|ExecutionSequence`
    (:`then_0`
      (`KismetSystemLibrary.Delay` 0.7)
      (`self.PlayIdle`))
    (:`then_1`
      (`KismetSystemLibrary.Delay` 0.2)
      (`/Game/Rehabilitation/Blueprints/VRGameInstance_BP.Success` (`/Game/Rehabilitation/Blueprints/MiscUtils/MiscUtils_BP.GetVRGameInstance`))
      (`self.SpawnRing`))))

(event `StartGame`
  (bind _vrgameinstance (`/Game/Rehabilitation/Blueprints/MiscUtils/MiscUtils_BP.GetVRGameInstance`))
  (if (not (`/Game/Rehabilitation/Blueprints/VRGameInstance_BP.IsGameStart` _vrgameinstance))
    (set `/Game/Rehabilitation/Blueprints/VRGameInstance_BP.IsGameStart` true _vrgameinstance)
    (set `self.IsPassRing` false)
    (`/Game/Rehabilitation/Blueprints/VRGameInstance_BP.Init` _vrgameinstance)
    (`self.SpawnRing`)
    (`self.SpawnBall`)
    (`self.PlayIdle`)))

(event `FinishGame`
  (bind _vrgameinstance (`/Game/Rehabilitation/Blueprints/MiscUtils/MiscUtils_BP.GetVRGameInstance`))
  (`|ExecutionSequence`
    (:`then_0`
      (`KismetSystemLibrary.PrintString` "Finish Game")
      (set `/Game/Rehabilitation/Blueprints/VRGameInstance_BP.IsGameStart` false _vrgameinstance)
      (`|ExecutionSequence`
        (:`then_0`
          (bind _ringobject (`self.RingObject`)
            (:`then`
              (`self.K2_DestroyActor` _ringobject))
            (:`else`)))))
    (:`then_1`
      (if (<= (`/Game/Rehabilitation/Blueprints/VRGameInstance_BP.GoalCount` _vrgameinstance) (`/Game/Rehabilitation/Blueprints/VRGameInstance_BP.SuccessCount` _vrgameinstance))
        (`SkeletalMeshComponent.PlayAnimation` (`self.SkeletalMesh`) "/Game/Tiny_Dragon/Animations/Anim_Dra_Jump.Anim_Dra_Jump" false)
        (`KismetSystemLibrary.Delay` 1.0)
        (`SkeletalMeshComponent.PlayAnimation` (`self.SkeletalMesh`) "/Game/Tiny_Dragon/Animations/Anim_Dra_Jump.Anim_Dra_Jump" false)
        (`KismetSystemLibrary.Delay` 1.0)
        (`SkeletalMeshComponent.PlayAnimation` (`self.SkeletalMesh`) "/Game/Tiny_Dragon/Animations/Anim_Dra_Fly_Fire.Anim_Dra_Fly_Fire" true)
        (`KismetSystemLibrary.Delay` 0.7)
        (`self.PlayIdle`)
        (else
          (`SkeletalMeshComponent.PlayAnimation` (`self.SkeletalMesh`) "/Game/Tiny_Dragon/Animations/Anim_Dra_Die.Anim_Dra_Die" false))))))

(event `InitData`
  (`/Game/Rehabilitation/Blueprints/VRGameInstance_BP.Init` (`/Game/Rehabilitation/Blueprints/MiscUtils/MiscUtils_BP.GetVRGameInstance`)))

(fn `UserConstructionScript`)